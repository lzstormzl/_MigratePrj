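; BP_PreviewCharacter is a preview character that showcases the MegaTauntsPack03 taunt animations by playing them in sequence.
; Two seconds after BeginPlay, PlayAnim plays the montage at the current AnimNo in the Animations array on the skeletal mesh.
; When a montage completes, it increments the index and calls PlayAnim again, with no bounds check or wrap-around.
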(event `self.ReceiveBeginPlay`
  (`KismetSystemLibrary.Delay` 2.0)
  (`self.PlayAnim`))

(event `PlayAnim`
  (`|PlayMontage` (`self.SkeletalMesh`) (`|GetArrayItem` (`self.Animations`) (`self.AnimNo`))
    (:`OnCompleted`
      (`/Engine/EditorBlueprintResources/StandardMacros.IncrementInt` (`self.AnimNo`)
        (:`  `
          (`self.PlayAnim`))))))

(fn `UserConstructionScript`)
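; Afterimage effect actor for MazeLong that mimics a character's pose, then fades out and destroys itself.
; For its first half second, Tick copies poses from source meshes onto its Base, Hair and Vay meshes, restarting both timelines whenever the base source is valid.
; The timelines drive glow and opacity through a shared Material Parameter Collection.
; Fade completion spawns an ending Niagara effect; the other timeline triggers delayed destruction.
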(event `self.ReceiveBeginPlay`
  (`|ExecutionSequence`
    (:`then_0`
      (set `self.MaxCopyTime` 0.5))
    (:`then_1`
      (set `self.CopyTime` 0.0))))

(event `self.ReceiveTick`
  (params (DeltaSeconds :type "Float (single-precision)"))
  (set `self.CopyTime` (+ (`self.CopyTime`) (`GameplayStatics.GetWorldDeltaSeconds`)))
  (if (< (`self.CopyTime`) (`self.MaxCopyTime`))
    (`|ExecutionSequence`
      (:`then_0`
        (bind _basetocopy (`self.BaseToCopy`)
          (:`then`
            (`PoseableMeshComponent.CopyPoseFromSkeletalComponent` (`self.Base`) _basetocopy)
            (`|ExecutionSequence`
              (:`then_0`
                (bind (_direction _opacity) (`Timeline|Timeline` :!via `PlayFromStart`)
                  (:`Update`
                    (`KismetMaterialLibrary.SetScalarParameterValue` "/Game/_MazeLong/Fx/MPC_MazeLongFX.MPC_MazeLongFX" "LightEff" _opacity))
                  (:`Finished`
                    (`KismetSystemLibrary.Delay` 0.2)
                    (`self.K2_DestroyActor`))))
              (:`then_1`
                (bind (_direction_2 _opacity_2) (`Timeline|Fade` :!via `PlayFromStart`)
                  (:`Update`
                    (`KismetMaterialLibrary.SetScalarParameterValue` "/Game/_MazeLong/Fx/MPC_MazeLongFX.MPC_MazeLongFX" "Opacity" _opacity_2))
                  (:`Finished`
                    (`NiagaraFunctionLibrary.SpawnSystemAttached` "/Game/_MazeLong/Fx/WaterForm/NS_MazeL_End_AfterImage.NS_MazeL_End_AfterImage" (`self.Base`) "None" (0.0 0.0 0.0) (struct) "KeepRelativeOffset"))))))
          (:`else`)))
      (:`then_1`
        (bind _hair_to_copy (`self.Hair to Copy`)
          (:`then`
            (`PoseableMeshComponent.CopyPoseFromSkeletalComponent` (`self.Hair`) _hair_to_copy))
          (:`else`)))
      (:`then_2`
        (bind _vay_to_copy (`self.Vay to Copy`)
          (:`then`
            (`PoseableMeshComponent.CopyPoseFromSkeletalComponent` (`self.Vay`) _vay_to_copy))
          (:`else`))))))

(fn `UserConstructionScript`)